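; BP_FinishPoint is a finish trigger that despawns NPCs reaching it.
; When a BP_NPC overlaps its trigger box, it stores the NPC, stops its task, and plays a despawn particle effect and sound.
; After a one-second delay it turns the effect off and destroys the stored NPC, which is held in a single variable across the delay.
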(event `self.ReceiveBeginPlay`
  (`ActorComponent.Deactivate` (`self.Particle Despawn`)))

(event `self.TriggerBox.OnComponentBeginOverlap`
  (params (OverlappedComponent :type "PrimitiveComponent Object Reference") (OtherActor :type "Actor Object Reference") (OtherComp :type "PrimitiveComponent Object Reference") (OtherBodyIndex :type Integer) (bFromSweep :type Boolean) (SweepResult :type "HitResult Structure (by ref)"))
  (bind _asbp_npc (cast `/Game/Exercise/NPC/BP_NPC` OtherActor))
  (bind _output_get (set `self.TargetNPC` _asbp_npc))
  (`/Game/Exercise/NPC/BP_NPC.TaskToStop` _output_get)
  (`ActorComponent.Activate` (`self.Particle Despawn`) false)
  (`GameplayStatics.PlaySoundAtLocation` (`self.DespawnSound`) (`SceneComponent.K2_GetComponentLocation` (`self.Particle Despawn`)) (struct) 0.5 1.0 0.5 null null null)
  (`KismetSystemLibrary.Delay` 1.0)
  (`ActorComponent.Deactivate` (`self.Particle Despawn`))
  (`self.K2_DestroyActor` (`self.TargetNPC`)))

(fn `UserConstructionScript`)