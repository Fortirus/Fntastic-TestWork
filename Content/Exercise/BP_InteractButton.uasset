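; Clickable world button that spawns an actor at a spawn point and, if it is a BP_NPC, tasks it to move to a target point.
; BeginPlay uses vertical line traces to find surface locations under both points and moves the spawn particle effect to the start.
; Cursor hover tints the mesh.
; Clicking spawns the actor, hands the NPC its movement type, plays particles and sound, then blocks reactivation for a cooldown.
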(event `self.ReceiveBeginPlay`
  (bind _finishlocation (`self.FinishLocation`))
  (`|ExecutionSequence`
    (:`then_0`
      (set `self.FinishLocation` (`self.K2_GetActorLocation` (`self.SpawnPoint`))) ; Spawn First
      (bind _outhit (`KismetSystemLibrary.LineTraceSingle` :`Start` (+ _finishlocation (0.0 0.0 150.0)) :`End` (+ _finishlocation (0.0 0.0 -100.0)) :`TraceChannel` "TraceTypeQuery1" :`DrawTime` 10.0 :!label _label))
      (set `self.FinishLocation` (`.Location` (`GameplayStatics.BreakHitResult` _outhit))))
    (:`then_1`
      (set `self.StartLocation` (`self.FinishLocation`))
      (set `self.FinishLocation` (`self.K2_GetActorLocation` (`self.TargetPont`)))
      (goto _label))
    (:`then_2`
      (`SceneComponent.K2_SetWorldLocation` (`self.Particle SpawnEffect`) (`self.StartLocation`) false false))))

(event `self.Collision Box.OnBeginCursorOver`
  (params (TouchedComponent :type "PrimitiveComponent Object Reference"))
  (set `self.isHovered` true)
  (`MeshComponent.SetVectorParameterValueOnMaterials` (`self.Mesh`) "Color" (`KismetMathLibrary.Conv_LinearColorToVector` (struct :`R` 1.0 :`B` 0.539998 :`A` 1.0))))

(event `self.Collision Box.OnEndCursorOver`
  (params (TouchedComponent :type "PrimitiveComponent Object Reference"))
  (set `self.isHovered` false)
  (`MeshComponent.SetVectorParameterValueOnMaterials` (`self.Mesh`) "Color" (`KismetMathLibrary.Conv_LinearColorToVector` (struct :`R` 1.0 :`G` 1.0 :`B` 1.0 :`A` 1.0))))

(event `self.Collision Box.OnClicked`
  (params (TouchedComponent :type "PrimitiveComponent Object Reference") (ButtonPressed :type "Key Structure"))
  (if (not (`self.isActivated`))
    (set `self.isActivated` true)
    (`self.TrySpawnActor`)
    (`KismetSystemLibrary.Delay` (`self.InteractCD`))
    (set `self.isActivated` false)))

(fn `TrySpawnActor`
  (locals (NewLocalVar_0 :type "Controller Object Reference"))
  (bind _startlocation (`self.StartLocation`))
  (bind _returnvalue (`|SpawnActorFromClass` (`self.SpawnActorClass`) (`KismetMathLibrary.MakeTransform` (+ (`self.StartLocation`) (0.0 0.0 30.0))) "AdjustIfPossibleButAlwaysSpawn" "OverrideRootScale" null null))
  (bind _asbp_npc (cast `/Game/Exercise/NPC/BP_NPC` _returnvalue))
  (`/Game/Exercise/NPC/BP_NPC.TaskToMove` _asbp_npc (`self.FinishLocation`) _startlocation (`self.SpawnActorMovementType`))
  (`ActorComponent.Activate` (`self.Particle SpawnEffect`) false)
  (`GameplayStatics.PlaySoundAtLocation` (`self.SpawnSound`) _startlocation (struct) 0.5 1.5 0.0 null null null))

(fn `UserConstructionScript`
  (`MeshComponent.SetVectorParameterValueOnMaterials` (`self.Mesh`) "Color" (`KismetMathLibrary.Conv_LinearColorToVector` (struct :`R` 1.0 :`G` 1.0 :`B` 1.0 :`A` 1.0))))