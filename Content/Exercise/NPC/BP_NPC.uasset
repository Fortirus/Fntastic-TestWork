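; BP_NPC is an NPC, animated by Fox_AnimBP, that walks to a given location in one of several movement styles.
; TaskToMove stores start and finish points, starts a SimpleMoveToLocation, and for types other than JustWalk runs CheckMovement, a self-calling delayed loop that pauses or briefly reverses movement.
; TaskToStop clears IsActive, which gates further moves through the IfActive macro, and flags the anim blueprint to rest.
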(event `Check Movement`
  (`self.IfActive`
    (:`Yes`
      (switch `/Game/Exercise/NPC/ENUM_MovementTypes` (`self.Movement Type`)
        (:`NewEnumerator1`
          ;[1 1 1] Walk and Stop
          (`KismetSystemLibrary.Delay` 1.0)
          (`self.IfActive`
            (:`Yes`
              (`Controller.StopMovement` (`self.GetController`))
              (`KismetSystemLibrary.Delay` 0.5)
              (`self.StartMoving`)
              (`self.Check Movement`))))
        (:`NewEnumerator2`
          ;[1 1 1] Walk and Reverse
          (`KismetSystemLibrary.Delay` 1.0)
          (`self.IfActive`
            (:`Yes`
              (set `self.Target Location` (`self.Start Location`))
              (`self.StartMoving`)
              (`KismetSystemLibrary.Delay` 0.5)
              (set `self.Target Location` (`self.Finish Location`))
              (`self.StartMoving`)
              (`self.Check Movement`))))))))

(fn `StartMoving`
  (`self.IfActive`
    (:`Yes`
      (`AIBlueprintHelperLibrary.SimpleMoveToLocation` (`self.GetController`) (`self.Target Location`)))))

(fn `TaskToMove`
  (params (TargetLocation :type "Vector Structure") (StartLocation :type "Vector Structure") (MovementType :type "/Game/Exercise/NPC/ENUM_MovementTypes Enum" :default "NewEnumerator0"))
  (`|ExecutionSequence`
    (:`then_0`
      (set `self.Target Location` TargetLocation)
      (set `self.Finish Location` TargetLocation)
      (set `self.Start Location` StartLocation)
      (set `self.Movement Type` MovementType)
      (set `self.isActive` true)
      (`self.StartMoving`))
    (:`then_1`
      (if (`|EnumInequality` (`self.Movement Type`) "NewEnumerator0")
        (`self.Check Movement`)))))

(fn `TaskToStop`
  (set `self.isActive` false)
  (bind _asfox_anim_bp (cast `/Game/AnimalVarietyPack/Fox/Fox_AnimBP` (`SkeletalMeshComponent.GetAnimInstance` (`self.Mesh`))))
  (set `/Game/AnimalVarietyPack/Fox/Fox_AnimBP.isGoingToRest` true _asfox_anim_bp) ; To play the Rest animation
)

(fn `UserConstructionScript`)